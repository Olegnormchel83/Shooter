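; Weapon pickup actor that looks up its drop info by item name from the game instance on BeginPlay.
; InitActor builds its look from that info, keeping either a static or skeletal mesh and an optional particle effect, destroying unused components.
; On character overlap it tries to add the weapon to the inventory, otherwise starts a weapon switch on the character.
; Leaving the sphere ends that switch.
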(event OnComponentEndOverlap(Sphere)
  (params (OverlappedComponent :type Primitive%20Component%20Object%20Reference) (OtherActor :type Actor%20Object%20Reference) (OtherComp :type Primitive%20Component%20Object%20Reference) (OtherBodyIndex :type Integer))
  (bind _asbp_character (Utilities|Casting|CastToBP_Character OtherActor))
  (Default|EndSwitchWeapon _asbp_character))

(event EventBeginPlay
  (bind _itemname (Variables|Default|GetItemName))
  (|CallParentFunction)
  (if (Utilities|Name|NotEqual(Name) _itemname "None")
    (bind _asbp_game_instance (Utilities|Casting|CastToBP_GameInstance (Game|GetGameInstance)))
    (bind (_outinfo _returnvalue) (Class|TPSGameInstance|GetDropItemInfobyName _asbp_game_instance _itemname))
    (if _returnvalue
      (bind _output_get (Variables|Default|SetWeaponInfo _outinfo))
      (CallFunction|InitActor _output_get))))

(event Collision|EventActorBeginOverlap
  (params (OtherActor :type Actor%20Object%20Reference))
  (|CallParentFunction OtherActor) ; This node is disabled and will not be called.\nDrag off pins to build functionality.
)

(event EventTick
  (params (DeltaSeconds :type Float%20%28single-precision%29))
  (|CallParentFunction DeltaSeconds) ; This node is disabled and will not be called.\nDrag off pins to build functionality.
)

(event EventOverlapCharacter
  (params (InentoryComponent :type TPS%20Inventory%20Component%20Object%20Reference))
  (|CallParentFunction InentoryComponent)
  (bind _returnvalue (Class|TPSInventoryComponent|TryGetWeapontoInventory InentoryComponent (.WeaponInfo (Utilities|Struct|BreakDropItem (Variables|Default|GetWeaponInfo)))))
  (if _returnvalue
    (CallFunction|PickUpSuccess)
    (else
      (bind _asbp_character (Utilities|Casting|CastToBP_Character (Components|GetOwner InentoryComponent)))
      (Default|StartSwitchWeapon _asbp_character self))))

(fn ConstructionScript
  (|CallParentFunction))

(fn InitActor
  (params (ActorInfo :type Drop%20Item%20Structure))
  (bind _staticmesh (Variables|Default|GetStaticMesh))
  (bind _skeletalmesh (Variables|Default|GetSkeletalMesh))
  (bind _output_get (Variables|Default|SetActor%20Info ActorInfo))
  (Utilities|FlowControl|Sequence
    (:then_0
      (Utilities|IsValid (.WeaponStaticMesh (Utilities|Struct|BreakDropItem _output_get))
        (:Is%20Valid
          (Components|DestroyComponent (Variables|Default|GetSkeletalMesh))
          (Components|StaticMesh|SetStaticMesh _staticmesh (.WeaponStaticMesh (Utilities|Struct|BreakDropItem _output_get)))
          (Transformation|SetRelativeLocation _staticmesh (.location (.Offset (Utilities|Struct|BreakDropItem _output_get))) false false)
          (Transformation|SetRelativeScale3D _staticmesh (.DropWeaponScale (Utilities|Struct|BreakDropItem _output_get))))
        (:Is%20Not%20Valid
          (Utilities|IsValid (.WeaponSkeletalMesh (Utilities|Struct|BreakDropItem _output_get))
            (:Is%20Valid
              (Components|DestroyComponent (Variables|Default|GetStaticMesh))
              (Class|SkinnedMeshComponent|SetSkeletalMesh _skeletalmesh (.WeaponSkeletalMesh (Utilities|Struct|BreakDropItem _output_get)) true)
              (Transformation|SetRelativeLocation _skeletalmesh (.location (.Offset (Utilities|Struct|BreakDropItem _output_get))) false false)
              (Transformation|SetRelativeScale3D _skeletalmesh (.DropWeaponScale (Utilities|Struct|BreakDropItem _output_get)))))))
      (Variables|Default|SetItemName (.NameItem (Utilities|Struct|BreakWeaponSlot (.WeaponInfo (Utilities|Struct|BreakDropItem _output_get)))) :!label _label)
      (Variables|Default|SetWeaponInfo (Variables|Default|GetActor%20Info)))
    (:then_1
      (Utilities|IsValid (.ParticleSystem (Utilities|Struct|BreakDropItem _output_get))
        (:Is%20Valid
          (Effects|Components|ParticleSystem|SetTemplate (Variables|Default|GetParticleSystem) (.ParticleSystem (Utilities|Struct|BreakDropItem _output_get)))
          (Transformation|SetRelativeScale3D (Variables|Default|GetParticleSystem) (.DropItemParticleScale (Utilities|Struct|BreakDropItem _output_get)))
          (goto _label))
        (:Is%20Not%20Valid
          (Components|DestroyComponent (Variables|Default|GetParticleSystem)))))))