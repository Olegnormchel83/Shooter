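; Lift actor that fades the camera out and carries its platform vertically when BP_Character enters its box trigger.
; The fade always runs and holds on overlap, while the move only runs if CanLiftMove is set.
; Moving snaps the door to a new relative location and plays a timeline that drives the platform's Z.
; The side walls, back wall and door are hidden at BeginPlay.
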(event OnComponentBeginOverlap(BoxCollider)
  (params (OverlappedComponent :type Primitive%20Component%20Object%20Reference) (OtherActor :type Actor%20Object%20Reference) (OtherComp :type Primitive%20Component%20Object%20Reference) (OtherBodyIndex :type Integer) (bFromSweep :type Boolean) (SweepResult :type Hit%20Result%20Structure%20%28by%20ref%29))
  (Utilities|Casting|CastToBP_Character OtherActor)
  (Utilities|FlowControl|Sequence
    (:then_0
      (CameraFades|StartCameraFade :self (Game|GetPlayerCameraManager 0) :ToAlpha 1.0 :Duration (Variables|Default|GetCameraFadeDuration) :bHoldWhenFinished true))
    (:then_1
      (if (Variables|Default|GetbCanLiftMove)
        (CallFunction|Move)))))

(event Custom|Move
  (Transformation|SetRelativeLocation (Variables|Default|GetLiftDoor) (Variables|Default|GetNew%20DoorLocation) false false)
  (bind _zoffset (Timeline|LiftTimeline Play)
    (:Update
      (Transformation|SetRelativeLocation (Variables|Default|GetPlatform) (Math|Vector|MakeVector 0.0 0.0 _zoffset) false false))))

(event EventBeginPlay
  (CallFunction|SetInvistoLiftWalls))

(event Collision|EventActorBeginOverlap
  (params (OtherActor :type Actor%20Object%20Reference)))

(event EventTick
  (params (DeltaSeconds :type Float%20%28single-precision%29)))

(fn ConstructionScript)

(fn SetInvistoLiftWalls
  (Rendering|SetVisibility (Variables|Default|GetWallLeft) false false)
  (Rendering|SetVisibility (Variables|Default|GetWallRight) false false)
  (Rendering|SetVisibility (Variables|Default|GetWallBack) false false)
  (Rendering|SetVisibility (Variables|Default|GetLiftDoor) false false))