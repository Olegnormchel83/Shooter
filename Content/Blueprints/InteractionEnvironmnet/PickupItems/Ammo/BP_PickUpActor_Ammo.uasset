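; Ammo pickup actor that adds ammo of a configured weapon type to the overlapping character's inventory component.
; On BeginPlay, InitActor picks a mesh and aura particle by weapon type and applies configured transforms, destroying either component when no asset exists, as with RocketLauncher.
; The parent's OverlapCharacter event checks whether the inventory can take that ammo, then changes the slot value and calls PickUpSuccess.
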(event EventBeginPlay
  (|CallParentFunction)
  (CallFunction|InitActor))

(event Collision|EventActorBeginOverlap
  (params (OtherActor :type Actor%20Object%20Reference))
  (|CallParentFunction OtherActor) ; This node is disabled and will not be called.\nDrag off pins to build functionality.
)

(event EventTick
  (params (DeltaSeconds :type Float%20%28single-precision%29))
  (|CallParentFunction DeltaSeconds) ; This node is disabled and will not be called.\nDrag off pins to build functionality.
)

(event EventOverlapCharacter
  (params (InentoryComponent :type TPS%20Inventory%20Component%20Object%20Reference))
  (bind _weapontypeammo (Variables|Default|GetWeaponTypeAmmo))
  (|CallParentFunction InentoryComponent)
  (bind _returnvalue (Class|TPSInventoryComponent|CheckCanTakeAmmo InentoryComponent _weapontypeammo))
  (if _returnvalue
    (Class|TPSInventoryComponent|AmmoSlotChangeValue InentoryComponent _weapontypeammo (Variables|Default|GetCout))
    (CallFunction|PickUpSuccess)))

(fn ConstructionScript
  (|CallParentFunction))

(fn InitActor
  (bind _weapontypeammo (Variables|Default|GetWeaponTypeAmmo))
  (bind _staticmesh (Variables|Default|GetStaticMesh))
  (bind _particlesystem (Variables|Default|GetParticleSystem))
  (bind _returnvalue (Utilities|Select :Index _weapontypeammo :RifleType "/Game/Blueprints/InteractionEnvironmnet/PickupItems/Ammo/Meshes/SM_AssaultRifle_Pickup.SM_AssaultRifle_Pickup" :ShotgunType "/Game/Blueprints/InteractionEnvironmnet/PickupItems/Ammo/Meshes/SM_Shotgun_Pickup.SM_Shotgun_Pickup" :SniperType "/Game/Blueprints/InteractionEnvironmnet/PickupItems/Ammo/Meshes/SM_SniperRifle_Pickup.SM_SniperRifle_Pickup" :GrenadeLauncherType "/Game/Blueprints/InteractionEnvironmnet/PickupItems/Ammo/Meshes/SM_GrenadeLauncher_Pickup.SM_GrenadeLauncher_Pickup" :RocketLauncherType 0))
  (bind _returnvalue_2 (Utilities|Select :Index _weapontypeammo :RifleType "/Game/Particles/PickupItemsAuras/P_RifleAura.P_RifleAura" :ShotgunType "/Game/Particles/PickupItemsAuras/P_ShotgunAura.P_ShotgunAura" :SniperType "/Game/Particles/PickupItemsAuras/P_SniperRifleAura.P_SniperRifleAura" :GrenadeLauncherType "/Game/Particles/PickupItemsAuras/P_GrenadeLauncherAura.P_GrenadeLauncherAura" :RocketLauncherType 0))
  (Utilities|FlowControl|Sequence
    (:then_0
      (Utilities|IsValid _returnvalue
        (:Is%20Valid
          (Components|StaticMesh|SetStaticMesh _staticmesh _returnvalue)
          (Transformation|SetRelativeLocation _staticmesh "0, 0, 0" false false)
          (Transformation|SetRelativeScale3D _staticmesh (Variables|Default|GetStaticMeshScale))
          (Transformation|SetRelativeRotation _staticmesh (Variables|Default|GetStaticMeshRotation) false false))
        (:Is%20Not%20Valid
          (Components|DestroyComponent _staticmesh))))
    (:then_1
      (Utilities|IsValid _returnvalue_2
        (:Is%20Valid
          (Effects|Components|ParticleSystem|SetTemplate _particlesystem _returnvalue_2)
          (Transformation|SetRelativeScale3D _particlesystem (Variables|Default|GetParticleScale)))
        (:Is%20Not%20Valid
          (Components|DestroyComponent _particlesystem))))))