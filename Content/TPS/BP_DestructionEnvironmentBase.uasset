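; Base Blueprint for destructible environment props in the TPS game, which take damage and are destroyed when their health runs out.
; Any damage feeds the TPSHealth component, whose health changes spawn a damage display actor near a local offset with slight random scatter.
; Radial damage from a ProjectileDefault applies that projectile's effect according to the mesh material's physical surface type.
; The component's death event calls Death, which destroys the actor.
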(event OnDead(TPSHealth)
  (CallFunction|Death))

(event OnHealthChanged(TPSHealth)
  (params (Health :type Float%20%28single-precision%29) (Damage :type Float%20%28single-precision%29))
  (bind _returnvalue (Game|SpawnActorfromClass "/Game/TPS/DisplayDamageActor.DisplayDamageActor_C" (Math|Transform|MakeTransform (+ (+ (Math|Vector|MakeVector (Math|Random|RandomFloatinRange -15.0 15.0) (Math|Random|RandomFloatinRange -15.0 15.0) 0.0) (Variables|Default|GetLocalPointToSpawnDamage)) (Transformation|GetActorLocation))) "AlwaysSpawn" 0 0))
  (Default|InitDisplayDamageActor _returnvalue Damage Health))

(event EventBeginPlay)

(event Collision|EventActorBeginOverlap
  (params (OtherActor :type Actor%20Object%20Reference)))

(event EventTick
  (params (DeltaSeconds :type Float%20%28single-precision%29)))

(event Game|Damage|EventAnyDamage
  (params (Damage :type Float%20%28single-precision%29) (DamageType :type Damage%20Type%20Object%20Reference) (InstigatedBy :type Controller%20Object%20Reference) (DamageCauser :type Actor%20Object%20Reference))
  (Class|TPSHealthComponent|ChangeHealthValue (Variables|Default|GetTPSHealth) (* -1 Damage)))

(event Game|Damage|EventRadialDamage
  (params (DamageReceived :type Float%20%28single-precision%29) (DamageType :type Damage%20Type%20Object%20Reference) (Origin :type Vector :default "0, 0, 0") (HitInfo :type Hit%20Result%20Structure%20%28by%20ref%29) (InstigatedBy :type Controller%20Object%20Reference) (DamageCauser :type Actor%20Object%20Reference))
  (bind _asprojectile_default (Utilities|Casting|CastToProjectileDefault DamageCauser))
  (Class|Types|AddEffectbySurfaceType self (.Effect (Utilities|Struct|BreakProjectileInfo (Variables|/Script/TPS.ProjectileDefault|GetProjectileSettings _asprojectile_default))) (Variables|/Script/PhysicsCore.PhysicalMaterial|GetSurfaceType (Class|MaterialInterface|GetPhysicalMaterial (Rendering|Material|GetMaterial (Variables|Default|GetStaticMesh) 0)))))

(fn ConstructionScript)

(fn Death
  (Actor|DestroyActor))