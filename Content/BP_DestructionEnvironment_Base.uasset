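; Base actor for destructible environment objects that take damage and are destroyed when their health runs out.
; AnyDamage passes negated damage to the TPSHealth component, whose health-change event spawns a display actor at a randomly jittered offset, showing damage and current health.
; TPSHealth's OnDead calls Death, which prints a debug message and destroys the actor.
; Death sound and particle spawns are unconnected placeholders with no assets set.
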(event OnHealthChanged(TPSHealth)
  (params (Health :type Float%20%28single-precision%29) (Damage :type Float%20%28single-precision%29))
  (bind _returnvalue (Game|SpawnActorfromClass "/Game/DisplayDamageActor.DisplayDamageActor_C" (Math|Transform|MakeTransform (+ (+ (Math|Vector|MakeVector (Math|Random|RandomFloatinRange -1e+01 1e+01) (Math|Random|RandomFloatinRange -1e+01 1e+01) 0.0) (Variables|Default|GetLocalPointSpawnHealthNumber)) (Transformation|GetActorLocation))) "AlwaysSpawn" 0 0))
  (Default|InitDisplayDamageActor _returnvalue Damage Health))

(event OnDead(TPSHealth)
  (CallFunction|Death))

(event EventBeginPlay)

(event Collision|EventActorBeginOverlap
  (params (OtherActor :type Actor%20Object%20Reference)))

(event EventTick
  (params (DeltaSeconds :type Float%20%28single-precision%29)))

(event Game|Damage|EventAnyDamage
  (params (Damage :type Float%20%28single-precision%29) (DamageType :type Damage%20Type%20Object%20Reference) (InstigatedBy :type Controller%20Object%20Reference) (DamageCauser :type Actor%20Object%20Reference))
  (Class|TPSHealthComponent|ChangeHealthValue (Variables|Default|GetTPSHealth) (* Damage -1.0)))

(event Game|Damage|EventPointDamage
  (params (Damage :type Float%20%28single-precision%29) (DamageType :type Damage%20Type%20Object%20Reference) (HitLocation :type Vector :default "0, 0, 0") (HitNormal :type Vector :default "0, 0, 0") (HitComponent :type Primitive%20Component%20Object%20Reference) (BoneName :type Name :default "None") (ShotFromDirection :type Vector :default "0, 0, 0") (InstigatedBy :type Controller%20Object%20Reference) (DamageCauser :type Actor%20Object%20Reference) (HitInfo :type Hit%20Result%20Structure%20%28by%20ref%29)))

(event Game|Damage|EventRadialDamage
  (params (DamageReceived :type Float%20%28single-precision%29) (DamageType :type Damage%20Type%20Object%20Reference) (Origin :type Vector :default "0, 0, 0") (HitInfo :type Hit%20Result%20Structure%20%28by%20ref%29) (InstigatedBy :type Controller%20Object%20Reference) (DamageCauser :type Actor%20Object%20Reference)))

(fn ConstructionScript)

(fn Death
  (Development|PrintString "I'm Dead" true true "(R=1.000000,G=0.000000,B=0.787000,A=1.000000)")
  (Actor|DestroyActor))